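; BP_AISpawner is a placed actor that spawns its share of each enemy wave at random reachable navmesh points around itself.
; It binds SpawnAI to the FPS game mode's RespawnEnemies event and divides the wave's enemy count by the spawner count.
; Early waves use only basic enemies, later ones pick random classes, and every tenth wave is skipped.
; A ProxDetector overlap tracks player proximity in ShouldSpawn, but SpawnAI never checks it.
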(event `self.ReceiveBeginPlay`
  (bind _asbp_fpsgame_mode_base (cast `/Game/BP/BP_FPSGameModeBase` (`GameplayStatics.GetGameMode`)))
  (bind _output_get (set `self.As BP FPSGame Mode Base` _asbp_fpsgame_mode_base))
  (add `/Game/BP/BP_FPSGameModeBase.RespawnEnemies` _output_get (delegate `Spawn AI`))
  (bind _outactors (`GameplayStatics.GetAllActorsOfClass` "BP_AISpawner_C"))
  (set `self.number of spawners` (`KismetArrayLibrary.Array_Length` _outactors)))

(event `Spawn AI`
  (bind _as_bp_fpsgame_mode_base (`self.As BP FPSGame Mode Base`))
  (bind _randomlocation (`NavigationSystemV1.K2_GetRandomReachablePointInRadius` (`self.K2_GetActorLocation`) 1000.0 null null))
  (bind _randomlocation_2 (`NavigationSystemV1.K2_GetRandomReachablePointInRadius` (`self.K2_GetActorLocation`) 1000.0 null null))
  (bind _wavenum (`/Game/BP/BP_FPSGameModeBase.WaveNum` _as_bp_fpsgame_mode_base))
  ;[1 1 1] Spawn AI if Player is close and their should be enemies spawned
  (if (not (== (mod _wavenum 10) 0))
    (for _ (range (+ (/ (`/Game/BP/BP_FPSGameModeBase.EnemiesThisWave` _as_bp_fpsgame_mode_base) (`self.number of spawners`)) 1))
      (if (< _wavenum 3)
        (`|SpawnActorFromClass` "/Game/BP/Actors/AI/BP_BasicEnemy.BP_BasicEnemy_C" (`KismetMathLibrary.MakeTransform` (`KismetMathLibrary.MakeVector` (.x _randomlocation_2) (.y _randomlocation_2) (.z _randomlocation_2)) (`self.K2_GetActorRotation`)) "AdjustIfPossibleButAlwaysSpawn" "MultiplyWithRoot" null null)
        (else
          (`|SpawnActorFromClass` (`KismetArrayLibrary.Array_Random` (`self.Class`)) (`KismetMathLibrary.MakeTransform` (`KismetMathLibrary.MakeVector` (.x _randomlocation) (.y _randomlocation) (.z _randomlocation)) (`self.K2_GetActorRotation`)) "AdjustIfPossibleButAlwaysSpawn" "MultiplyWithRoot" null null))))))

(event `self.Prox detector.OnComponentBeginOverlap`
  (params (OverlappedComponent :type "PrimitiveComponent Object Reference") (OtherActor :type "Actor Object Reference") (OtherComp :type "PrimitiveComponent Object Reference") (OtherBodyIndex :type Integer) (bFromSweep :type Boolean) (SweepResult :type "HitResult Structure (by ref)"))
  ;[1 1 1] Check if player is close enough, using a box so its room shaped and because its quicker to do than making the code for BSP-based spawning, although the map itself will be made with the BSP tools, idk if theres a way to add actors to it
  (set `self.bShouldSpawn` (`self.ActorHasTag` OtherActor "Player")))

(event `self.Prox detector.OnComponentEndOverlap`
  (params (OverlappedComponent :type "PrimitiveComponent Object Reference") (OtherActor :type "Actor Object Reference") (OtherComp :type "PrimitiveComponent Object Reference") (OtherBodyIndex :type Integer))
  ;[1 1 1] Check if player is close enough, using a box so its room shaped and because its quicker to do than making the code for BSP-based spawning, although the map itself will be made with the BSP tools, idk if theres a way to add actors to it
  (if (`self.ActorHasTag` OtherActor "Player")
    (set `self.bShouldSpawn` false)))

(fn `UserConstructionScript`)