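; BP_Anom is a damageable enemy actor that can spawn other enemies around itself in the FPS game.
; It registers with BP_FPSGameModeBase's living-enemy count on BeginPlay and subtracts incoming damage from its Health.
; At zero health it decrements that count, has the game mode check the enemy amount, and destroys itself.
; Its Spawn event, not called within this graph, spawns a random EnemiesToSpawn class at a nearby reachable point.
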(event `self.ReceiveBeginPlay`
  (add `self.OnTakeAnyDamage` (delegate `OnTakeAnyDamage_Event`))
  (bind _asbp_fpsgame_mode_base (cast `/Game/BP/BP_FPSGameModeBase` (`GameplayStatics.GetGameMode`)))
  (bind _output_get (set `self.As BP FPSGame Mode Base` _asbp_fpsgame_mode_base))
  (`/Engine/EditorBlueprintResources/StandardMacros.IncrementInt` (`/Game/BP/BP_FPSGameModeBase.EnemiesAlive` _output_get)))

(event `OnTakeAnyDamage_Event` :!signature `self.OnTakeAnyDamage`
  (params (DamagedActor :type "Actor Object Reference") (Damage :type "Float (single-precision)") (DamageType :type "DamageType Object Reference") (InstigatedBy :type "Controller Object Reference") (DamageCauser :type "Actor Object Reference"))
  (bind _as_bp_fpsgame_mode_base (`self.As BP FPSGame Mode Base`))
  (bind _output_get (set `self.Health` (- (`self.Health`) Damage)))
  (if (<= _output_get 0.0)
    (`/Engine/EditorBlueprintResources/StandardMacros.DecrementInt` (`/Game/BP/BP_FPSGameModeBase.EnemiesAlive` _as_bp_fpsgame_mode_base)
      (:`  `
        (`/Game/BP/BP_FPSGameModeBase.CheckEnemyAmount` _as_bp_fpsgame_mode_base)
        (`self.K2_DestroyActor`)))))

(event `Spawn`
  (`|SpawnActorFromClass` (`KismetArrayLibrary.Array_Random` (`self.Enemies to Spawn`)) (`KismetMathLibrary.MakeTransform` (`NavigationSystemV1.K2_GetRandomReachablePointInRadius` (`self.K2_GetActorLocation`) 1000.0 null null)) "Undefined" "MultiplyWithRoot" null null))

(fn `UserConstructionScript`)