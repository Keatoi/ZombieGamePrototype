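; BP_Crawler is a wave-based FPS enemy whose health scales with the wave number and which registers in the game mode's alive count.
; Pawn sensing of the player class BP_test sets a line-of-sight blackboard key.
; Attack sphere-traces forward and damages that player class.
; On death it detaches its controller, ragdolls, updates the game mode's enemy count, occasionally drops a random pickup, then destroys itself after a delay.
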(event `self.ReceiveBeginPlay`
  (add `self.OnTakeAnyDamage` (delegate `OnTakeAnyDamage_Event`))
  (bind _asbp_fpsgame_mode_base (cast `/Game/BP/BP_FPSGameModeBase` (`GameplayStatics.GetGameMode`)))
  (bind _output_get (set `self.As BP FPSGame Mode Base` _asbp_fpsgame_mode_base))
  (`/Engine/EditorBlueprintResources/StandardMacros.IncrementInt` (`/Game/BP/BP_FPSGameModeBase.EnemiesAlive` _output_get)
    (:`  `
      (set `self.Health` (* (`self.Health`) (`/Game/BP/BP_FPSGameModeBase.WaveNum` _output_get))))))

(event `self.ReceiveTick`
  (params (DeltaSeconds :type "Float (single-precision)")))

(event `OnTakeAnyDamage_Event` :!signature `self.OnTakeAnyDamage`
  (params (DamagedActor :type "Actor Object Reference") (Damage :type "Float (single-precision)") (DamageType :type "DamageType Object Reference") (InstigatedBy :type "Controller Object Reference") (DamageCauser :type "Actor Object Reference"))
  (bind _as_bp_fpsgame_mode_base (`self.As BP FPSGame Mode Base`))
  ;[1 1 1] Take Damage
  (set `self.Health` (- (`self.Health`) Damage))
  ;[1 1 1] Health Check
  (if (<= (`self.Health`) 0.0)
    (`self.DetachFromControllerPendingDestroy`)
    (`PrimitiveComponent.SetSimulatePhysics` (`self.Mesh`) true)
    (`/Engine/EditorBlueprintResources/StandardMacros.DecrementInt` (`/Game/BP/BP_FPSGameModeBase.EnemiesAlive` _as_bp_fpsgame_mode_base)
      (:`  `
        (`/Game/BP/BP_FPSGameModeBase.CheckEnemyAmount` _as_bp_fpsgame_mode_base)
        (if (`KismetMathLibrary.RandomBoolWithWeight` 0.15)
          ;[1 1 1] Rand Pickup Spawn 15% of the time
          (`|SpawnActorFromClass` (`KismetArrayLibrary.Array_Random` (`self.PickUpArr`)) (`self.GetTransform`) "Undefined" "MultiplyWithRoot" null null))
        (`KismetSystemLibrary.Delay` 3.0)
        (`self.K2_DestroyActor`)))))

(event `self.PawnSensing.OnSeePawn`
  (params (Pawn :type "Pawn Object Reference"))
  ;[1 1 1] Sight Check
  (cast `/Game/BP/Actors/Player/BP_test` Pawn)
  (`BlackboardComponent.SetValueAsBool` (`AIBlueprintHelperLibrary.GetBlackboard` (`AIBlueprintHelperLibrary.GetAIController` self)) "bHasLOS?" true)
  (set `self.bHasLos` true))

(event `Attack`
  (bind _returnvalue (`self.K2_GetActorLocation`))
  (bind (_outhit _returnvalue_2) (`KismetSystemLibrary.SphereTraceSingleForObjects` _returnvalue (+ _returnvalue (* (`KismetMathLibrary.GetForwardVector` (`self.K2_GetActorRotation`)) 250.0)) 100.0 (`|MakeArray` "ObjectTypeQuery3" :!type "EObjectTypeQuery Enum")))
  (if _returnvalue_2
    (bind (_bblockinghit _binitialoverlap _time _distance _location _impactpoint _normal _impactnormal _physmat _hitactor) (`GameplayStatics.BreakHitResult` _outhit))
    (cast `/Game/BP/Actors/Player/BP_test` _hitactor)
    (`GameplayStatics.ApplyDamage` _hitactor (`self.Base Damage`))))

(fn `UserConstructionScript`)