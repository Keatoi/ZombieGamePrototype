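; BP_Generator is a map actor that the player can activate by spending Dosh.
; On BeginPlay it caches the BP_test player and creates an interact widget, which its Box overlap shows and hides.
; IA_Interact deducts Cost and sets Activated if the stored overlap actor is the player, which is never cleared on exit.
; The cost check only tests that Cost is positive, not that the player can afford it.
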(event `self.ReceiveBeginPlay`
  (bind _returnvalue (`|CreateWidget` "/Game/UserInterface/WBP_Interact.WBP_Interact_C"))
  (set `self.InteractUI` _returnvalue)
  (bind _asbp_test (cast `/Game/BP/Actors/Player/BP_test` (`GameplayStatics.GetPlayerCharacter` 0)))
  (set `self.As BP Test` _asbp_test)
  (set `self.bActivated` false))

(event `self.ReceiveTick`
  (params (DeltaSeconds :type "Float (single-precision)")))

(event `self.Box.OnComponentBeginOverlap`
  (params (OverlappedComponent :type "PrimitiveComponent Object Reference") (OtherActor :type "Actor Object Reference") (OtherComp :type "PrimitiveComponent Object Reference") (OtherBodyIndex :type Integer) (bFromSweep :type Boolean) (SweepResult :type "HitResult Structure (by ref)"))
  (bind _as_bp_test (`self.As BP Test`))
  (bind _returnvalue (== OtherActor _as_bp_test))
  (`KismetSystemLibrary.PrintString` (`KismetStringLibrary.Conv_BoolToString` _returnvalue))
  (if _returnvalue
    (`UserWidget.AddToViewport` (`self.InteractUI`) 0)
    (set `self.Other Actor` _as_bp_test)))

(event `self.Box.OnComponentEndOverlap`
  (params (OverlappedComponent :type "PrimitiveComponent Object Reference") (OtherActor :type "Actor Object Reference") (OtherComp :type "PrimitiveComponent Object Reference") (OtherBodyIndex :type Integer))
  (if (== OtherActor (`self.As BP Test`))
    (`Widget.RemoveFromParent` (`self.InteractUI`))))

(event `EnhancedInput|/Game/Input/Actions/IA_Interact`
  (params (ActionValue :type Boolean) (ElapsedSeconds :type "Float (double-precision)") (TriggeredSeconds :type "Float (double-precision)") (InputAction :type "InputAction Object Reference" :default "/Game/Input/Actions/IA_Interact.IA_Interact"))
  (bind _as_bp_test (`self.As BP Test`))
  (bind _other_actor (`self.Other Actor`))
  (bind _dosh (`PlayerChar.Dosh` _as_bp_test))
  (bind _returnvalue (- _dosh (`self.Cost`)))
  (:`Started`
    (`/Engine/EditorBlueprintResources/StandardMacros.IsValid` _other_actor
      (:`Is Valid`
        (if (== _other_actor (`self.As BP Test`))
          (if (< _returnvalue _dosh)
            (set `PlayerChar.Dosh` _returnvalue _as_bp_test)
            (set `self.bActivated` true)))))))

(fn `UserConstructionScript`)