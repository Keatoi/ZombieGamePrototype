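; BP_MedKit is a pickup actor that adds one med kit to the player when touched.
; On BeginPlay it casts the player character to BP_test and caches it.
; When that character overlaps the Sphere component, it increments the character's MedKits count, plays the Flashlight_Switch sound at its location and destroys itself.
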(event `self.ReceiveBeginPlay`
  (bind _asbp_test (cast `/Game/BP/Actors/Player/BP_test` (`GameplayStatics.GetPlayerCharacter` 0)))
  (set `self.As BP Test` _asbp_test))

(event `self.ReceiveTick`
  (params (DeltaSeconds :type "Float (single-precision)")))

(event `self.Sphere.OnComponentBeginOverlap`
  (params (OverlappedComponent :type "PrimitiveComponent Object Reference") (OtherActor :type "Actor Object Reference") (OtherComp :type "PrimitiveComponent Object Reference") (OtherBodyIndex :type Integer) (bFromSweep :type Boolean) (SweepResult :type "HitResult Structure (by ref)"))
  (if (== OtherActor (`self.As BP Test`))
    (`/Engine/EditorBlueprintResources/StandardMacros.IncrementInt` (`PlayerChar.MedKits` (`self.As BP Test`))
      (:`  `
        (`GameplayStatics.PlaySoundAtLocation` "/Engine/VREditor/Sounds/UI/Flashlight_Switch.Flashlight_Switch" (`self.K2_GetActorLocation`) (struct) 1.0 1.0 0.0 null null null null)
        (`self.K2_DestroyActor`)))))

(fn `UserConstructionScript`)