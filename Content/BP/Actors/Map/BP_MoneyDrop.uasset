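; BP_MoneyDrop is a cash pickup that adds money to the game mode when the player touches it.
; On BeginPlay it caches the player character as BP_test and the BP_FPSGameModeBase game mode.
; Its static mesh spins by a fixed amount every tick, independent of delta time.
; Overlapping its sphere with the player adds CashToAdd to the game mode's Cash, plays a sound and destroys the actor.
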(event `self.ReceiveBeginPlay`
  (bind _asbp_test (cast `/Game/BP/Actors/Player/BP_test` (`GameplayStatics.GetPlayerCharacter` 0)))
  (set `self.As BP Test` _asbp_test)
  (bind _asbp_fpsgame_mode_base (cast `/Game/BP/BP_FPSGameModeBase` (`GameplayStatics.GetGameMode`)))
  (set `self.As BP FPSGame Mode Base` _asbp_fpsgame_mode_base))

(event `self.ReceiveTick`
  (params (DeltaSeconds :type "Float (single-precision)"))
  (`SceneComponent.K2_AddLocalRotation` (`self.StaticMesh`) (struct :`Yaw` 5.0) false false))

(event `self.Sphere.OnComponentBeginOverlap`
  (params (OverlappedComponent :type "PrimitiveComponent Object Reference") (OtherActor :type "Actor Object Reference") (OtherComp :type "PrimitiveComponent Object Reference") (OtherBodyIndex :type Integer) (bFromSweep :type Boolean) (SweepResult :type "HitResult Structure (by ref)"))
  (bind _as_bp_fpsgame_mode_base (`self.As BP FPSGame Mode Base`))
  (if (== OtherActor (`self.As BP Test`))
    (set `FPSGameModeBase.Cash` (+ (`FPSGameModeBase.Cash` _as_bp_fpsgame_mode_base) (`self.CashToAdd`)) _as_bp_fpsgame_mode_base)
    (`GameplayStatics.PlaySoundAtLocation` "/Engine/VREditor/Sounds/UI/Flashlight_Switch.Flashlight_Switch" (`self.K2_GetActorLocation`) (struct) 1.0 1.0 0.0 null null null null)
    (`self.K2_DestroyActor`)))

(fn `UserConstructionScript`)