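; First-person player Blueprint that handles the HUD, two weapon slots, grenade throwing, health and game over.
; BeginPlay spawns and socket-attaches two weapons to the FPS arms; equip inputs swap them between grip and unused sockets.
; Reload and grenade aim hide the arms; releasing launches a physics grenade.
; Damage hits armour before health, death opens the game-over level, and GetGripSocket converts the gun's grip into hand-bone space.
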(event `EnhancedInput|/Game/Input/Actions/IA_Reload`
  (params (ActionValue :type Boolean) (ElapsedSeconds :type "Float (double-precision)") (TriggeredSeconds :type "Float (double-precision)") (InputAction :type "InputAction Object Reference" :default "/Game/Input/Actions/IA_Reload.IA_Reload"))
  (:`Started`
    (`SceneComponent.SetVisibility` (`self.FPSArms`) false true)
    (`KismetSystemLibrary.Delay` (`AWeapon.ReloadTime` (`self.CurrentWeapon`)))
    (`SceneComponent.SetVisibility` (`self.FPSArms`) true true)))

(event `self.ReceiveBeginPlay`
  (bind _returnvalue (`|CreateWidget` "/Game/UserInterface/WBP_Player.WBP_Player_C" (`GameplayStatics.GetPlayerController` 0)))
  (`UserWidget.AddToViewport` _returnvalue 0)
  (`self.Spawn Attach Weapon` "/Game/BP/Actors/Weapon/BP_testweapon.BP_testweapon_C")
  (`self.Spawn Attach Weapon` "/Game/BP/Actors/Weapon/BP_Val.BP_Val_C")
  (`self.Set CurrentWeapon` (`self.PrimaryWeapon`))
  (add `self.OnTakeAnyDamage` (delegate `OnTakeAnyDamage_Event`)))

(event `OnTakeAnyDamage_Event` :!signature `self.OnTakeAnyDamage`
  (params (DamagedActor :type "Actor Object Reference") (Damage :type "Float (single-precision)") (DamageType :type "DamageType Object Reference") (InstigatedBy :type "Controller Object Reference") (DamageCauser :type "Actor Object Reference"))
  (if (> (`self.Armour`) 0.0)
    ;[1 1 1] Damage Armour if it exists
    (set `self.Armour` (`KismetMathLibrary.MapRangeClamped` (- (`self.Armour`) Damage) 0.0 100.0 0.0 100.0))
    (else
      ;[1 1 1] Subtract from Health if no armour
      (`GameplayStatics.PlaySound2D` "/Game/Assets/Sounds/Jack_Menhorn_FPS_Placeholder/bodyimpact_jack_01.bodyimpact_jack_01" 1.0 1.0 0.0 null null)
      (set `self.Health` (- (`self.Health`) Damage))))
  (if (<= (`self.Health`) 0.0)
    (`GameplayStatics.PlaySound2D` (`KismetArrayLibrary.Array_Random` (`self.Death Sound`)) 1.0 1.0 0.0 null null)
    (`GameplayStatics.OpenLevelBySoftObjectPtr` "/Game/MAPS/LVL_GameOver.LVL_GameOver")))

(event `EnhancedInput|/Game/Input/Actions/IA_Grenade`
  (params (ActionValue :type Boolean) (ElapsedSeconds :type "Float (double-precision)") (TriggeredSeconds :type "Float (double-precision)") (InputAction :type "InputAction Object Reference" :default "/Game/Input/Actions/IA_Grenade.IA_Grenade"))
  (:`Started`
    (if (> (`self.Grenade Amount`) 0)
      (set `self.bIsAiming?` true)
      (`SceneComponent.SetVisibility` (`self.FPSArms`) false true)
      (set `AWeapon.bCanFire` false (`self.CurrentWeapon`))))
  (:`Completed`
    (if (> (`self.Grenade Amount`) 0)
      (set `self.bIsAiming?` false)
      (bind _returnvalue (`|SpawnActorFromClass` "/Game/BP/Actors/Weapon/BP_Grenade.BP_Grenade_C" (`KismetMathLibrary.MakeTransform` (`SceneComponent.K2_GetComponentLocation` (`self.GrenREF`)) (`self.K2_GetActorRotation`)) "Undefined" "MultiplyWithRoot" null null))
      (`PrimitiveComponent.SetPhysicsLinearVelocity` (`/Game/BP/Actors/Weapon/BP_Grenade.Sphere` _returnvalue) (* (`KismetMathLibrary.GetDirectionUnitVector` (`self.K2_GetActorLocation`) (`self.K2_GetActorLocation` _returnvalue)) (`self.ThrowSpeed`)) false "None")
      (`SceneComponent.SetVisibility` (`self.FPSArms`) true true)
      (set `AWeapon.bCanFire` true (`self.CurrentWeapon`))
      (`/Engine/EditorBlueprintResources/StandardMacros.DecrementInt` (`self.Grenade Amount`)))))

(event `EnhancedInput|/Game/Input/Actions/IA_EquipPrim`
  (params (ActionValue :type Boolean) (ElapsedSeconds :type "Float (double-precision)") (TriggeredSeconds :type "Float (double-precision)") (InputAction :type "InputAction Object Reference" :default "/Game/Input/Actions/IA_EquipPrim.IA_EquipPrim"))
  (:`Started`
    (`KismetSystemLibrary.PrintString` "1")
    (`self.swap to primary`)))

(event `EnhancedInput|/Game/Input/Actions/IA_EquipSecond`
  (params (ActionValue :type Boolean) (ElapsedSeconds :type "Float (double-precision)") (TriggeredSeconds :type "Float (double-precision)") (InputAction :type "InputAction Object Reference" :default "/Game/Input/Actions/IA_EquipSecond.IA_EquipSecond"))
  (:`Started`
    (`KismetSystemLibrary.PrintString` "2")
    (`self.swap to seconday`)))

(fn `Get GripSocket`
  (returns (SocketLoc :type "Transform Structure"))
  (bind _currentweapon (`self.CurrentWeapon`))
  (`/Engine/EditorBlueprintResources/StandardMacros.IsValid` _currentweapon
    (:`Is Valid`
      (bind _asbp_testweapon (cast `/Game/BP/Actors/Weapon/BP_testweapon` _currentweapon))
      (bind (_returnvalue_location _returnvalue_rotation) (`KismetMathLibrary.BreakTransform` (`SceneComponent.GetSocketTransform` (`AWeapon.GunSK` _asbp_testweapon) "GunGrip" "RTS_World")))
      (bind (_outposition _outrotation) (`SkinnedMeshComponent.TransformToBoneSpace` (`self.FPSArms`) "hand_r" _returnvalue_location _returnvalue_rotation))
      (return (`KismetMathLibrary.MakeTransform` _outposition _outrotation)))
    (:`Is Not Valid`
      (`KismetSystemLibrary.PrintString` "not valid"))))

(fn `Set CurrentWeapon`
  (params (WeaponToSet :type "AWeapon Object Reference"))
  (bind _output_get (set `self.CurrentWeapon` WeaponToSet))
  (`KismetSystemLibrary.PrintString` (`KismetSystemLibrary.GetObjectName` _output_get)))

(fn `Spawn Attach Weapon`
  (params (WeaponClass :type "AWeapon Class Reference"))
  (bind _primaryweapon (`self.PrimaryWeapon`))
  (bind _backupweapon (`self.BackupWeapon`))
  (bind _returnvalue (`GameplayStatics.GetActorOfClass` WeaponClass))
  (if (`|EnumEquality` (`AWeapon.WeaponType` _returnvalue) "EPrimary")
    (`/Engine/EditorBlueprintResources/StandardMacros.IsValid` _primaryweapon
      (:`Is Valid`
        (`self.K2_DestroyActor` _primaryweapon)
        (set `self.PrimaryWeapon` null))
      (:`Is Not Valid`
        _))
    (else
      (`/Engine/EditorBlueprintResources/StandardMacros.IsValid` _backupweapon
        (:`Is Valid`
          (`self.K2_DestroyActor` _backupweapon)
          (set `self.BackupWeapon` null))
        (:`Is Not Valid`
          _))))
  (bind _returnvalue_2 (`|SpawnActorFromClass` WeaponClass (`KismetMathLibrary.MakeTransform` (0.0 0.0 0.0)) "Undefined" "MultiplyWithRoot" null null))
  (if (`|EnumEquality` (`AWeapon.WeaponType` _returnvalue_2) "EPrimary")
    (bind _output_get (set `self.PrimaryWeapon` _returnvalue_2))
    (`self.K2_AttachToComponent` _output_get (`self.FPSArms`) "GripPoint" "KeepRelative" "KeepRelative" "KeepRelative" true)
    (else
      (bind _output_get_2 (set `self.BackupWeapon` _returnvalue_2))
      (`self.K2_AttachToComponent` _output_get_2 (`self.FPSArms`) "UnusedPoint" "KeepRelative" "KeepRelative" "KeepRelative" true))))

(fn `swap to primary`
  (`/Engine/EditorBlueprintResources/StandardMacros.IsValid` (`self.PrimaryWeapon`)
    (:`Is Valid`
      (`/Engine/EditorBlueprintResources/StandardMacros.IsValid` (`self.BackupWeapon`)
        (:`Is Valid`
          (if (== (`SceneComponent.GetAttachSocketName` (`AWeapon.GunSK` (`self.PrimaryWeapon`))) "UnusedPoint")
            (`KismetSystemLibrary.PrintString` "sec Equiped")
            (`SceneComponent.SetVisibility` (`self.FPSArms`) false true)
            (`self.K2_DetachFromActor` (`self.PrimaryWeapon`) "KeepRelative" "KeepRelative" "KeepRelative")
            (`self.K2_DetachFromActor` (`self.BackupWeapon`) "KeepRelative" "KeepRelative" "KeepRelative")
            (`self.K2_AttachToComponent` (`self.PrimaryWeapon`) (`self.FPSArms`) "GripPoint" "KeepRelative" "KeepRelative" "KeepRelative" true)
            (`self.K2_AttachToComponent` (`self.BackupWeapon`) (`self.FPSArms`) "UnusedPoint" "KeepRelative" "KeepRelative" "KeepRelative" true)
            (`SceneComponent.SetVisibility` (`self.FPSArms`) true true)
            (`self.Set CurrentWeapon` (`self.PrimaryWeapon`))
            (else
              (`KismetSystemLibrary.PrintString` "pri equiped"))))))))

(fn `swap to seconday`
  (`/Engine/EditorBlueprintResources/StandardMacros.IsValid` (`self.PrimaryWeapon`)
    (:`Is Valid`
      (`/Engine/EditorBlueprintResources/StandardMacros.IsValid` (`self.BackupWeapon`)
        (:`Is Valid`
          (if (== (`SceneComponent.GetAttachSocketName` (`AWeapon.GunSK` (`self.BackupWeapon`))) "UnusedPoint")
            (`KismetSystemLibrary.PrintString` "Pri Equiped")
            (`SceneComponent.SetVisibility` (`self.FPSArms`) false true)
            (`self.K2_DetachFromActor` (`self.BackupWeapon`) "KeepRelative" "KeepRelative" "KeepRelative")
            (`self.K2_DetachFromActor` (`self.PrimaryWeapon`) "KeepRelative" "KeepRelative" "KeepRelative")
            (`self.K2_AttachToComponent` (`self.BackupWeapon`) (`self.FPSArms`) "GripPoint" "KeepRelative" "KeepRelative" "KeepRelative" true)
            (`self.K2_AttachToComponent` (`self.PrimaryWeapon`) (`self.FPSArms`) "UnusedPoint" "KeepRelative" "KeepRelative" "KeepRelative" true)
            (`SceneComponent.SetVisibility` (`self.FPSArms`) true true)
            (`self.Set CurrentWeapon` (`self.BackupWeapon`))
            (else
              (`KismetSystemLibrary.PrintString` "scdry equiped"))))))))

(fn `UserConstructionScript`)