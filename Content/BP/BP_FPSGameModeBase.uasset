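; Game mode for a wave-based zombie FPS that runs enemy waves and the game over transition.
; BeginPlay calls CallRespawnEnemies to start spawning, which is implemented outside this graph.
; When CheckEnemyAmount finds no enemies alive, it enlarges the enemy count, increments the wave with a sound, and respawns.
; HandleGameOver stores wave and Cash (as score) in ZombieInstance, then opens the game over level.
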(event `self.ReceiveBeginPlay`
  (`self.RespawnEnemies`))

(event `CheckEnemyAmount`
  (if (== (`self.EnemiesAlive`) 0)
    (set `self.EnemiesThisWave` (* (+ (`self.EnemiesThisWave`) (`self.WaveNum`)) 2))
    ;[1 1 1] increase wave then respawn AI
    (`self.StartNewWave`)
    (`self.RespawnEnemies`)))

(fn `HandleGameOver`
  ;[1 1 1] Set wave and score in the instance then open the game over level
  (bind _aszombie_instance (cast `/Game/BP/ZombieInstance` (`GameplayStatics.GetGameInstance`)))
  (bind _output_get (set `self.As Zombie Instance` _aszombie_instance))
  (set `/Game/BP/ZombieInstance.Wave` (`self.WaveNum`) _output_get)
  (set `/Game/BP/ZombieInstance.Score` (`self.Cash`) _output_get)
  (`GameplayStatics.OpenLevelBySoftObjectPtr` "/Game/MAPS/LVL_GameOver.LVL_GameOver"))

(fn `StartNewWave`
  (if true
    ;[1 1 1] Special Wave
    (`/Engine/EditorBlueprintResources/StandardMacros.IncrementInt` (`self.WaveNum`)
      (:`  `
        (`GameplayStatics.PlaySound2D` "/Game/Assets/Sounds/AmbientandUI/NewWave.NewWave" 1.0 1.0 0.0 null null)))))

(fn `UserConstructionScript`)